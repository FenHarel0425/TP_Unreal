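; BP_BombExplosion is a bomb actor that flashes as a countdown and then removes itself.
; On BeginPlay it creates two dynamic material instances on the Bomb mesh, a mine texture and a red gem material.
; It alternates between them at fixed delays, then destroys the actor right after the last switch to red.
; No damage, effects or overlap logic is implemented.
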(event `self.ReceiveBeginPlay`
  (bind _returnvalue (`PrimitiveComponent.CreateDynamicMaterialInstance` (`self.Bomb`) 0 "/Game/Models/Mine/M_TextureMines.M_TextureMines" "None"))
  (set `self.BombMaterial` _returnvalue)
  (bind _returnvalue_2 (`PrimitiveComponent.CreateDynamicMaterialInstance` (`self.Bomb`) 0 "/Game/Models/Mine/GemRed.GemRed" "None"))
  (set `self.BombMaterialBoom` _returnvalue_2)
  (`KismetSystemLibrary.Delay` 1.0)
  (`PrimitiveComponent.SetMaterial` (`self.Bomb`) 0 (`self.BombMaterialBoom`))
  (`KismetSystemLibrary.Delay` 1.0)
  (`PrimitiveComponent.SetMaterial` (`self.Bomb`) 0 (`self.BombMaterial`))
  (`KismetSystemLibrary.Delay` 1.0)
  (`PrimitiveComponent.SetMaterial` (`self.Bomb`) 0 (`self.BombMaterialBoom`))
  (`self.K2_DestroyActor`))

(fn `UserConstructionScript`)