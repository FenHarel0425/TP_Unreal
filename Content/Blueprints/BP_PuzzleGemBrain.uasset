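; BP_PuzzleGemBrain is the controller for a gem puzzle that opens a door.
; Shortly after BeginPlay it binds CheckPuzzle to each gem in Gems.
; Good events raise or lower ActivatedCount depending on whether PuzzleLight is active; reaching TotalCount turns that light green, destroys the door and plays a boom.
; A second bad event plays a denial sound, resets both counters and hides all gem lights.
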(event `self.ReceiveBeginPlay`
  (`KismetSystemLibrary.Delay` 0.2)
  (for _array_element (`self.Gems`)
    (add `/Game/Blueprints/BP_GEM.GemPuzzle` _array_element (delegate `CheckPuzzle`))))

(event `CheckPuzzle`
  (params (isGood :type Boolean))
  (if isGood
    (if (`ActorComponent.IsActive` (`/Game/Blueprints/BP_GemPuzzleLight.PointLight` (`self.PuzzleLight`)))
      (`/Engine/EditorBlueprintResources/StandardMacros.DecrementInt` (`self.ActivatedCount`)
        (:`  `
          _))
      (else
        (`/Engine/EditorBlueprintResources/StandardMacros.IncrementInt` (`self.ActivatedCount`)
          (:`  `
            _))))
    (if (>= (`self.ActivatedCount`) (`self.TotalCount`))
      (`LightComponent.SetLightColor` (`/Game/Blueprints/BP_GemPuzzleLight.PointLight` (`self.PuzzleLight`)) (struct :`R` 0.022202 :`G` 0.182292 :`B` 0.021486 :`A` 1.0) true)
      (`self.K2_DestroyActor` (`self.Door`))
      (`AudioComponent.Play` (`self.BoomSFX`) 0.0)
      (set `self.isDoorDestroyed` true))
    (else
      (`/Engine/EditorBlueprintResources/StandardMacros.IncrementInt` (`self.BadCount`)
        (:`  `
          (if (>= (`self.BadCount`) 2)
            (`AudioComponent.Play` (`self.Denied`) 0.0)
            (set `self.ActivatedCount` 0)
            (set `self.BadCount` 0)
            (for _array_element (`self.Gems`)
              (`SceneComponent.SetVisibility` (`/Game/Blueprints/BP_GEM.PointLight` _array_element) false false))))))))

(fn `UserConstructionScript`)