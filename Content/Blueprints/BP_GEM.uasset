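; BP_GEM is an interactable gem for a puzzle tied to a destructible door.
; While PuzzleBrain reports the door intact, each interaction toggles the point light, syncs IsTurnedOn to its visibility and plays the gem sound.
; It then fires GemPuzzle with the gem's IsGood flag.
; Once the door is destroyed, interaction does nothing.
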(event `self.Interacted`
  (if (not (`/Game/Blueprints/BP_PuzzleGemBrain.isDoorDestroyed` (`self.PuzzleBrain`)))
    (`SceneComponent.ToggleVisibility` (`self.PointLight`) false)
    (if (`SceneComponent.IsVisible` (`self.PointLight`))
      (set `self.isTurnedOn` true)
      (else
        (set `self.isTurnedOn` false)))
    (`AudioComponent.Play` (`self.SFX_Gem`) 0.0)
    (`self.GemPuzzle` (`self.isGood`))))

(fn `UserConstructionScript`
  (`parent.UserConstructionScript`))