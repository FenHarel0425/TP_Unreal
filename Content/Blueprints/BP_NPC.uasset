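; BP_NPC is a non-player character that shows dialogue lines in the game mode's MainUI panel.
; Interacted uses ArrayIndex to pick the Intro, OnGoing or Outro lines from DialogueAsset, then calls Talk to display the current line after a short delay.
; BeginPlay shows the cursor and binds Button1 to advance DialogueIndex, with no bounds check or reset.
; An older Intro-only sequence remains unconnected.
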(event `OnClicked_Event`
  (bind _asbp_third_person_game_mode (cast `/Game/ThirdPerson/Blueprints/BP_ThirdPersonGameMode` (`GameplayStatics.GetGameMode`)))
  (bind _mainui (`/Game/ThirdPerson/Blueprints/BP_ThirdPersonGameMode.MainUI` _asbp_third_person_game_mode))
  (`TextBlock.SetText` (`/Game/Blueprints/UMG/UMG_MainUI.TextDialogue` _mainui) (`|GetArrayItem` (`/Game/Blueprints/DataDialogue/BP_DA_Dialogue.Intro` (`self.DialogueAsset`)) 1))
  (add `Button.OnClicked` (`/Game/Blueprints/UMG/UMG_MainUI.Button1` _mainui) (delegate `CustomEvent`)))

(event `CustomEvent`
  (set `Widget.Visibility` "Hidden" (`/Game/Blueprints/UMG/UMG_MainUI.DialoguePanel` (`/Game/ThirdPerson/Blueprints/BP_ThirdPersonGameMode.MainUI` (stale `OnClicked_Event` _asbp_third_person_game_mode)))))

(event `Talk`
  (bind _asbp_third_person_game_mode (cast `/Game/ThirdPerson/Blueprints/BP_ThirdPersonGameMode` (`GameplayStatics.GetGameMode`)))
  (`KismetSystemLibrary.Delay` 1.0)
  (bind _mainui (`/Game/ThirdPerson/Blueprints/BP_ThirdPersonGameMode.MainUI` _asbp_third_person_game_mode))
  (set `Widget.Visibility` "Visible" (`/Game/Blueprints/UMG/UMG_MainUI.DialoguePanel` _mainui))
  (`TextBlock.SetText` (`/Game/Blueprints/UMG/UMG_MainUI.TextDialogue` _mainui) (`|GetArrayItem` (`self.CurrentDialogue`) (`self.DialogueIndex`))))

(event `self.Interacted`
  (bind _dialogueasset (`self.DialogueAsset`))
  (switch `int` (`self.ArrayIndex`)
    (:`0`
      (set `self.CurrentDialogue` (`/Game/Blueprints/DataDialogue/BP_DA_Dialogue.Intro` _dialogueasset)))
    (:`1`
      (set `self.CurrentDialogue` (`/Game/Blueprints/DataDialogue/BP_DA_Dialogue.OnGoing` _dialogueasset)))
    (:`2`
      (set `self.CurrentDialogue` (`/Game/Blueprints/DataDialogue/BP_DA_Dialogue.Outro` _dialogueasset))))
  (`self.Talk`))

(event `self.ReceiveBeginPlay`
  (`parent.ReceiveBeginPlay`)
  (bind _asbp_third_person_game_mode (cast `/Game/ThirdPerson/Blueprints/BP_ThirdPersonGameMode` (`GameplayStatics.GetGameMode`)))
  (add `Button.OnClicked` (`/Game/Blueprints/UMG/UMG_MainUI.Button1` (`/Game/ThirdPerson/Blueprints/BP_ThirdPersonGameMode.MainUI` _asbp_third_person_game_mode)) (delegate `OnClickedEvent`))
  (set `PlayerController.bShowMouseCursor` true (`GameplayStatics.GetPlayerController` 0)))

(event `OnClickedEvent`
  (bind _result (`/Engine/EditorBlueprintResources/StandardMacros.IncrementInt` (`self.DialogueIndex`))
    (:`  `
      (set `self.DialogueIndex` _result)
      (`self.Talk`))))

(fn `UserConstructionScript`
  (`parent.UserConstructionScript`))