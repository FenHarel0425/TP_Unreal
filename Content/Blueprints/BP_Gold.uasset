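; BP_Gold is a collectible gold pickup that responds to an Interacted event.
; The first interaction sets IsGoldCollected, plays the SFXGem sound and destroys the Cube and Bubble components, with the flag blocking repeat collection.
; The actor itself is not destroyed, and the graph awards no score or currency.
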(event `self.Interacted`
  (if (not (`self.isGoldCollected`))
    (set `self.isGoldCollected` true)
    (`AudioComponent.Play` (`self.SFX_Gem`) 0.0)
    (`ActorComponent.K2_DestroyComponent` (`self.Cube`))
    (`ActorComponent.K2_DestroyComponent` (`self.Bubble`))))

(fn `UserConstructionScript`
  (`parent.UserConstructionScript`))